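; Key-locked door that swings open for the first-person player and uses a light to signal access.
; BeginPlay caches the player character and puts a dynamic material instance on the light mesh.
; Entering the collision brightens the light, turning it green and playing the rotation Timeline if the player has the key, or red otherwise.
; Leaving restores the dim amber light and reverses the Timeline.
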(event `self.ReceiveBeginPlay`
  ;[0.15 0.6696 0.15 0.5] Setup
  (bind _asbp_first_person_character (cast `/Game/StarterContent/FirstPerson/Blueprints/BP_FirstPersonCharacter` (`GameplayStatics.GetPlayerCharacter` 0)))
  (set `self.BP First Person Character` _asbp_first_person_character)
  (bind _returnvalue (`KismetMaterialLibrary.CreateDynamicMaterialInstance` "/Game/MyContent/Materials/MI_Door_Light.MI_Door_Light"))
  (set `self.DynamicMaterial` _returnvalue)
  (`PrimitiveComponent.SetMaterial` (`self.SM_Light`) 0 (`self.DynamicMaterial`)))

(event `self.Collision.OnComponentBeginOverlap`
  (params (OverlappedComponent :type "PrimitiveComponent Object Reference") (OtherActor :type "Actor Object Reference") (OtherComp :type "PrimitiveComponent Object Reference") (OtherBodyIndex :type Integer) (bFromSweep :type Boolean) (SweepResult :type "HitResult Structure (by ref)"))
  (bind _dynamicmaterial (`self.DynamicMaterial`))
  ; Change Light
  (if (== OtherActor (`self.BP First Person Character`))
    (`MaterialInstanceDynamic.SetScalarParameterValue` _dynamicmaterial "Intensity" 100.0)
    (if (`/Game/StarterContent/FirstPerson/Blueprints/BP_FirstPersonCharacter.HasKey` (`self.BP First Person Character`))
      (`MaterialInstanceDynamic.SetVectorParameterValue` _dynamicmaterial "Colour" (struct :`G` 1.0 :`A` 1.0))
      ; Door Animation
      (bind (_direction _alpha) (`Timeline|Timeline` :!label _label)
        (:`Update`
          (`SceneComponent.K2_SetRelativeRotation` (`self.SM_Door`) (`KismetMathLibrary.RLerp` (struct) (struct :`Yaw` 90.0) _alpha) false false)))
      (else
        (`MaterialInstanceDynamic.SetVectorParameterValue` _dynamicmaterial "Colour" (struct :`R` 1.0 :`A` 1.0))))))

(event `self.Collision.OnComponentEndOverlap`
  (params (OverlappedComponent :type "PrimitiveComponent Object Reference") (OtherActor :type "Actor Object Reference") (OtherComp :type "PrimitiveComponent Object Reference") (OtherBodyIndex :type Integer))
  (bind _dynamicmaterial (`self.DynamicMaterial`))
  ; Return Light to Default
  (if (== OtherActor (`self.BP First Person Character`))
    (`MaterialInstanceDynamic.SetScalarParameterValue` _dynamicmaterial "Intensity" 1.0)
    (`MaterialInstanceDynamic.SetVectorParameterValue` _dynamicmaterial "Colour" (struct :`R` 1.0 :`G` 0.723055 :`B` 0.246201 :`A` 1.0))
    (goto _label :!via `Reverse`)))

(fn `UserConstructionScript`)